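; AC_Camera_System is a camera occlusion system that makes geometry between the camera and player character transparent.
; Each Tick, a Visibility line trace runs from the camera to the character's capsule, recording the hit component and its slot 0 material.
; While the first recorded component stays hit, it receives the Transparent material.
; A different hit or none applies the first saved material to all recorded components and clears both arrays.
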(event `self.ReceiveTick`
  (params (DeltaSeconds :type "Float (single-precision)"))
  (bind _outhit (`KismetSystemLibrary.LineTraceSingle` (`PlayerCameraManager.GetCameraLocation` (`GameplayStatics.GetPlayerCameraManager` 0)) (`SceneComponent.GetSocketLocation` (`Character.CapsuleComponent` (`GameplayStatics.GetPlayerCharacter` 0)) "None") "TraceTypeQuery1"))
  (if (`GameplayStatics.BreakHitResult` _outhit)
    (`KismetArrayLibrary.Array_Add` (`self.InitialHit`) (`.HitComponent` (`GameplayStatics.BreakHitResult` _outhit)))
    (if (== (`|GetArrayItem` (`self.InitialHit`)) (`|GetArrayItem` (`|MakeArray` (`.HitComponent` (`GameplayStatics.BreakHitResult` _outhit)))))
      (set `self.IsComponent` true)
      (else
        (set `self.IsComponent` false)))
    (if (`self.IsComponent`)
      (`KismetArrayLibrary.Array_Add` (`self.OriginalMaterial`) (`PrimitiveComponent.GetMaterial` (`.HitComponent` (`GameplayStatics.BreakHitResult` _outhit)) 0))
      (`PrimitiveComponent.SetMaterial` (`self.InitialHit`) 0 "/Camera_System/Transparent.Transparent")
      (else
        (`PrimitiveComponent.SetMaterial` (`self.InitialHit`) 0 (`|GetArrayItem` (`self.OriginalMaterial`)) :!label _label)
        (`KismetArrayLibrary.Array_Clear` (`self.OriginalMaterial`))
        (`KismetArrayLibrary.Array_Clear` (`self.InitialHit`))))
    (else
      (goto _label))))